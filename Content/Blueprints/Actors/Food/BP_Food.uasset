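; BP_Food is a food item actor that displays one of several Japanese dishes, or slop, chosen by its FoodType.
; SetFoodMesh maps each FoodType value to a static mesh and assigns it to the FoodMesh component.
; It runs from both the Construction Script and BeginPlay, so the mesh is set at construction and again when play starts.
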(event `self.ReceiveBeginPlay`
  (`parent.ReceiveBeginPlay`)
  (`self.SetFoodMesh`))

(fn `SetFoodMesh`
  (locals (NewFoodMesh :type "StaticMesh Object Reference"))
  (switch `EFoodType` (`self.FoodType`)
    (:`Dango`
      (set `local.NewFoodMesh` "/Game/Food/Food_Dango.Food_Dango"))
    (:`Wasabi`
      (set `local.NewFoodMesh` "/Game/Food/Food_Wasabi.Food_Wasabi"))
    (:`SalmonNigiri`
      (set `local.NewFoodMesh` "/Game/Food/Food_SalmonNigiri.Food_SalmonNigiri"))
    (:`EbiNigiri`
      (set `local.NewFoodMesh` "/Game/Food/Food_EbiNigiri.Food_EbiNigiri"))
    (:`OctopusNigiri`
      (set `local.NewFoodMesh` "/Game/Food/Food_OctopusNigiri.Food_OctopusNigiri"))
    (:`Ramen`
      (set `local.NewFoodMesh` "/Game/Food/Food_Ramen.Food_Ramen"))
    (:`SeaUrchinRoll`
      (set `local.NewFoodMesh` "/Game/Food/Food_SeaUrchinRoll.Food_SeaUrchinRoll"))
    (:`Slop`
      (set `local.NewFoodMesh` "/Game/Food/Food_Slop.Food_Slop")))
  (`StaticMeshComponent.SetStaticMesh` (`self.FoodMesh`) (`local.NewFoodMesh`)))

(fn `UserConstructionScript`
  (`parent.UserConstructionScript`)
  (`self.SetFoodMesh`))