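; BP_Ingredients is a food ingredient actor that displays a sushi-style ingredient such as rice, nori, fish or vegetables.
; The Construction Script switches on IngredientType, stores the matching static mesh in CurrentIngredientMesh and applies it to the IngredientMesh component.
; One Blueprint thus covers every ingredient variant, with the mesh resolved at construction.
; The Event Graph holds only disabled placeholder events, so the actor has no runtime logic there.
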(fn `UserConstructionScript`
  (locals (CurrentIngredientMesh :type "StaticMesh Object Reference"))
  (switch `EIngredientType` (`self.IngredientType`)
    (:`Avocado`
      (set `local.CurrentIngredientMesh` "/Game/Food/FoodIngredient_Avocado.FoodIngredient_Avocado"))
    (:`Crabsticks`
      (set `local.CurrentIngredientMesh` "/Game/Food/FoodIngredient_Crabsticks.FoodIngredient_Crabsticks"))
    (:`Cucumber`
      (set `local.CurrentIngredientMesh` "/Game/Food/FoodIngredient_Cucumber.FoodIngredient_Cucumber"))
    (:`Ebi`
      (set `local.CurrentIngredientMesh` "/Game/Food/FoodIngredient_Ebi.FoodIngredient_Ebi"))
    (:`Eel`
      (set `local.CurrentIngredientMesh` "/Game/Food/FoodIngredient_Eel.FoodIngredient_Eel"))
    (:`Fish`
      (set `local.CurrentIngredientMesh` "/Game/Food/FoodIngredient_Fish.FoodIngredient_Fish"))
    (:`FishFillet`
      (set `local.CurrentIngredientMesh` "/Game/Food/FoodIngredient_FishFillet.FoodIngredient_FishFillet"))
    (:`Flounder`
      (set `local.CurrentIngredientMesh` "/Game/Food/FoodIngredient_Flounder.FoodIngredient_Flounder"))
    (:`Mackerel`
      (set `local.CurrentIngredientMesh` "/Game/Food/FoodIngredient_Mackerel.FoodIngredient_Mackerel"))
    (:`Nori`
      (set `local.CurrentIngredientMesh` "/Game/Food/FoodIngredient_Nori.FoodIngredient_Nori"))
    (:`Octopus`
      (set `local.CurrentIngredientMesh` "/Game/Food/FoodIngredient_Octopus.FoodIngredient_Octopus"))
    (:`Rice`
      (set `local.CurrentIngredientMesh` "/Game/Food/FoodIngredient_Rice.FoodIngredient_Rice"))
    (:`Salmon`
      (set `local.CurrentIngredientMesh` "/Game/Food/FoodIngredient_Salmon.FoodIngredient_Salmon"))
    (:`SeaUrchin`
      (set `local.CurrentIngredientMesh` "/Game/Food/FoodIngredient_SeaUrchin.FoodIngredient_SeaUrchin")))
  (`StaticMeshComponent.SetStaticMesh` (`self.IngredientMesh`) (`local.CurrentIngredientMesh`)))